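; Teleporter actor that moves any Character entering its Box trigger to the location of a TeleportTarget actor.
; When ExitPoint is set, the construction script hides the Plane and BeginPlay disables the Box's overlap events, leaving it as a destination only.
; Tick spins the Plane continuously around yaw as a visual marker.
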(event OnComponentBeginOverlap(Box)
  (params (OverlappedComponent :type Primitive%20Component%20Object%20Reference) (OtherActor :type Actor%20Object%20Reference) (OtherComp :type Primitive%20Component%20Object%20Reference) (OtherBodyIndex :type Integer) (bFromSweep :type Boolean) (SweepResult :type Hit%20Result%20Structure%20%28by%20ref%29))
  (bind _ascharacter (Utilities|Casting|CastToCharacter OtherActor))
  (bind _teleporttarget (Variables|Default|GetTeleportTarget)
    (:then
      (Transformation|SetActorLocation _ascharacter (Transformation|GetActorLocation _teleporttarget) false true))
    (:else)))

(event EventBeginPlay
  (if (Variables|Default|GetExitPoint)
    (Variables|/Script/Engine.PrimitiveComponent|SetbGenerateOverlapEvents (Variables|Default|GetBox) false)))

(event Collision|EventActorBeginOverlap
  (params (OtherActor :type Actor%20Object%20Reference)))

(event EventTick
  (params (DeltaSeconds :type Float%20%28single-precision%29))
  (Transformation|AddRelativeRotation (Variables|Default|GetPlane) (Math|Rotator|MakeRotator 0.0 0.0 (* DeltaSeconds 1.8e+02)) false false))

(fn ConstructionScript
  (if (Variables|Default|GetExitPoint)
    (Rendering|SetVisibility (Variables|Default|GetPlane) false false)))