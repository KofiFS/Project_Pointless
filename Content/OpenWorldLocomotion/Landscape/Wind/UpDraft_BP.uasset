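; Wind updraft actor that lifts characters using the open-world locomotion gliding component.
; A timeline started on overlap updates each overlapping character, suspending its glide floor check until it leaves, and stops when none remain.
; In the required locomotion state, the Shaft launches characters along the actor's up vector at Strength.
; With StayTop enabled, the Top zone eases each character's stored Z velocity toward zero to hold them aloft.
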(event Collision|EventActorBeginOverlap
  (params (OtherActor :type Actor%20Object%20Reference))
  (bind _overlappingactors (Collision|GetOverlappingActors "/Script/Engine.Character" :!class /Script/Engine.Actor))
  (Utilities|Casting|CastToCharacter OtherActor)
  (Timeline|Timeline_0 PlayFromStart
    (:Update
      (if (> (Utilities|Array|Length _overlappingactors) 0)
        (for _array_element _overlappingactors
          (Utilities|IsValid (Actor|GetComponentbyClass _array_element "/Game/OpenWorldLocomotion/CharacterComponents/SystemComponents/OWL_Gliding_BP.OWL_Gliding_BP_C")
            (:Is%20Valid
              (Variables|/Game/OpenWorldLocomotion/CharacterComponents/SystemComponents/OWL_Gliding_BP.OWL_Gliding_BP_C|SetGlidingStartFloorCheck (Actor|GetComponentbyClass _array_element "/Game/OpenWorldLocomotion/CharacterComponents/SystemComponents/OWL_Gliding_BP.OWL_Gliding_BP_C") false)
              (if (Utilities|Enum|Equal(Enum) (Variables|/Game/OpenWorldLocomotion/CharacterComponents/OWL_BaseComponent_BP.OWL_BaseComponent_BP_C|GetLocomotionState (Variables|/Game/OpenWorldLocomotion/CharacterComponents/SystemComponents/ComponentClass/ComponentClass_BP.ComponentClass_BP_C|GetBaseComponent (Actor|GetComponentbyClass _array_element "/Game/OpenWorldLocomotion/CharacterComponents/SystemComponents/OWL_Gliding_BP.OWL_Gliding_BP_C"))) "NewEnumerator4")
                (if (Collision|IsOverlappingActor (Variables|Default|GetShaft) (.AsCharacter (Utilities|Casting|CastToCharacter _array_element)) :!class /Script/Engine.PrimitiveComponent)
                  (Default|GlidingLaunchCharacter (Actor|GetComponentbyClass _array_element "/Game/OpenWorldLocomotion/CharacterComponents/SystemComponents/OWL_Gliding_BP.OWL_Gliding_BP_C") 0.0 (* (Transformation|GetActorUpVector) (Variables|Default|GetStrength)) false true)
                  (Utilities|Map|Add (Variables|Default|GetVelocityZ) (.AsCharacter (Utilities|Casting|CastToCharacter _array_element)) (Variables|Default|GetStrength))
                  (elif (and (Collision|IsOverlappingActor (Variables|Default|GetTop) (.AsCharacter (Utilities|Casting|CastToCharacter _array_element)) :!class /Script/Engine.PrimitiveComponent) (Variables|Default|GetStayTop))
                    (Utilities|Map|Add (Variables|Default|GetVelocityZ) (.AsCharacter (Utilities|Casting|CastToCharacter _array_element)) (Math|Interpolation|FInterpTo (.Value (Utilities|Map|Find (Variables|Default|GetVelocityZ) (.AsCharacter (Utilities|Casting|CastToCharacter _array_element)))) 1e-06 (Utilities|Time|GetWorldDeltaSeconds) 5e+01))
                    (Default|GlidingLaunchCharacter (Actor|GetComponentbyClass _array_element "/Game/OpenWorldLocomotion/CharacterComponents/SystemComponents/OWL_Gliding_BP.OWL_Gliding_BP_C") 0.0 (Math|Vector|MakeVector 0.0 0.0 (Math|Interpolation|FInterpTo (.Value (Utilities|Map|Find (Variables|Default|GetVelocityZ) (.AsCharacter (Utilities|Casting|CastToCharacter _array_element)))) 1e-06 (Utilities|Time|GetWorldDeltaSeconds) 5e+01)) false true)))))))
        (else
          (Timeline|Timeline_0 Stop))))))

(event Collision|EventActorEndOverlap
  (params (OtherActor :type Actor%20Object%20Reference))
  (bind _returnvalue (Actor|GetComponentbyClass OtherActor "/Game/OpenWorldLocomotion/CharacterComponents/SystemComponents/OWL_Gliding_BP.OWL_Gliding_BP_C"))
  (Utilities|IsValid _returnvalue
    (:Is%20Valid
      (Variables|/Game/OpenWorldLocomotion/CharacterComponents/SystemComponents/OWL_Gliding_BP.OWL_Gliding_BP_C|SetGlidingStartFloorCheck _returnvalue true))))

(fn ConstructionScript)