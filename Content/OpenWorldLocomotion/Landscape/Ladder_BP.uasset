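; Ladder actor for the open world locomotion system that switches characters inside its volume into a climbing mode.
; On begin play or overlap, it passes its LadderData (self reference and step heights) to the character's OWL_Climbing_BP component and sets the mode.
; It also binds to that component's ChangeClimbingMode event, reapplying ladder mode while overlap lasts and unbinding otherwise.
; Leaving the volume resets the mode and unbinds.
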(event OnComponentBeginOverlap(ClimbingModeVolume)
  (params (OverlappedComponent :type Primitive%20Component%20Object%20Reference) (OtherActor :type Actor%20Object%20Reference) (OtherComp :type Primitive%20Component%20Object%20Reference) (OtherBodyIndex :type Integer) (bFromSweep :type Boolean) (SweepResult :type Hit%20Result%20Structure%20%28by%20ref%29))
  (bind _ascharacter (Utilities|Casting|CastToCharacter OtherActor))
  (Utilities|IsValid (Actor|GetComponentbyClass _ascharacter "/Game/OpenWorldLocomotion/CharacterComponents/SystemComponents/OWL_Climbing_BP.OWL_Climbing_BP_C")
    (:Is%20Valid
      (EventDispatchers|AssignChangeClimbingMode (Actor|GetComponentbyClass _ascharacter "/Game/OpenWorldLocomotion/CharacterComponents/SystemComponents/OWL_Climbing_BP.OWL_Climbing_BP_C") (EventDispatchers|CreateEvent :!event ChangeClimbingModeEvent))
      (Variables|/Game/OpenWorldLocomotion/CharacterComponents/SystemComponents/OWL_Climbing_BP.OWL_Climbing_BP_C|SetLadderData (Actor|GetComponentbyClass _ascharacter "/Game/OpenWorldLocomotion/CharacterComponents/SystemComponents/OWL_Climbing_BP.OWL_Climbing_BP_C") (Variables|Default|GetLadderData))
      (Variables|/Game/OpenWorldLocomotion/CharacterComponents/SystemComponents/OWL_Climbing_BP.OWL_Climbing_BP_C|SetClimbingMode (Actor|GetComponentbyClass _ascharacter "/Game/OpenWorldLocomotion/CharacterComponents/SystemComponents/OWL_Climbing_BP.OWL_Climbing_BP_C") "NewEnumerator1"))))

(event OnComponentEndOverlap(ClimbingModeVolume)
  (params (OverlappedComponent :type Primitive%20Component%20Object%20Reference) (OtherActor :type Actor%20Object%20Reference) (OtherComp :type Primitive%20Component%20Object%20Reference) (OtherBodyIndex :type Integer))
  (bind _ascharacter (Utilities|Casting|CastToCharacter OtherActor))
  (Utilities|IsValid (Actor|GetComponentbyClass _ascharacter "/Game/OpenWorldLocomotion/CharacterComponents/SystemComponents/OWL_Climbing_BP.OWL_Climbing_BP_C")
    (:Is%20Valid
      (Variables|/Game/OpenWorldLocomotion/CharacterComponents/SystemComponents/OWL_Climbing_BP.OWL_Climbing_BP_C|SetClimbingMode (Actor|GetComponentbyClass _ascharacter "/Game/OpenWorldLocomotion/CharacterComponents/SystemComponents/OWL_Climbing_BP.OWL_Climbing_BP_C") "NewEnumerator0")
      (EventDispatchers|UnbindEventfromChangeClimbingMode (Actor|GetComponentbyClass _ascharacter "/Game/OpenWorldLocomotion/CharacterComponents/SystemComponents/OWL_Climbing_BP.OWL_Climbing_BP_C") (EventDispatchers|CreateEvent :!event ChangeClimbingModeEvent)))))

(event EventBeginPlay
  (for _array_element (Collision|GetOverlappingActors (Variables|Default|GetClimbingModeVolume) "/Script/Engine.Character" :!class /Script/Engine.PrimitiveComponent)
    (Utilities|IsValid (Actor|GetComponentbyClass _array_element "/Game/OpenWorldLocomotion/CharacterComponents/SystemComponents/OWL_Climbing_BP.OWL_Climbing_BP_C")
      (:Is%20Valid
        (EventDispatchers|AssignChangeClimbingMode (Actor|GetComponentbyClass _array_element "/Game/OpenWorldLocomotion/CharacterComponents/SystemComponents/OWL_Climbing_BP.OWL_Climbing_BP_C") (EventDispatchers|CreateEvent :!event ChangeClimbingModeEvent))
        (Variables|/Game/OpenWorldLocomotion/CharacterComponents/SystemComponents/OWL_Climbing_BP.OWL_Climbing_BP_C|SetLadderData (Actor|GetComponentbyClass _array_element "/Game/OpenWorldLocomotion/CharacterComponents/SystemComponents/OWL_Climbing_BP.OWL_Climbing_BP_C") (Variables|Default|GetLadderData))
        (Variables|/Game/OpenWorldLocomotion/CharacterComponents/SystemComponents/OWL_Climbing_BP.OWL_Climbing_BP_C|SetClimbingMode (Actor|GetComponentbyClass _array_element "/Game/OpenWorldLocomotion/CharacterComponents/SystemComponents/OWL_Climbing_BP.OWL_Climbing_BP_C") "NewEnumerator1")))))

(fn ConstructionScript
  (Variables|Default|SetLadderData (Utilities|Struct|MakeLadderData_Struct self (.stepheight (Variables|Default|GetLadderData)) (.firststepheight (Variables|Default|GetLadderData)))))

(fn ChangeClimbingModeEvent
  (params (Ref%20Self :type OWL%20Climbing%20BP%20Object%20Reference))
  (if (Collision|IsOverlappingActor (Variables|Default|GetClimbingModeVolume) (Components|GetOwner Ref%20Self) :!class /Script/Engine.PrimitiveComponent)
    (Variables|/Game/OpenWorldLocomotion/CharacterComponents/SystemComponents/OWL_Climbing_BP.OWL_Climbing_BP_C|SetLadderData Ref%20Self (Variables|Default|GetLadderData))
    (Variables|/Game/OpenWorldLocomotion/CharacterComponents/SystemComponents/OWL_Climbing_BP.OWL_Climbing_BP_C|SetClimbingMode Ref%20Self "NewEnumerator1")
    (else
      (EventDispatchers|UnbindEventfromChangeClimbingMode Ref%20Self (EventDispatchers|CreateEvent :!event ChangeClimbingModeEvent)))))