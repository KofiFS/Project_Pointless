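; Moving object Blueprint that starts travelling along a list of points when a Character first overlaps its Box.
; A looping MoveComponentTo moves the StaticMesh at a set Velocity, pausing between points.
; The Return flag picks ping-pong or wrap-around order, with the actor's starting location inserted into the path.
; A separate trigger enables climbing on moving objects in OWL_Climbing_BP while the overlapping actor stays inside.
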(event OnComponentBeginOverlap(ClimbOnMovingObjectsTrigger)
  (params (OverlappedComponent :type Primitive%20Component%20Object%20Reference) (OtherActor :type Actor%20Object%20Reference) (OtherComp :type Primitive%20Component%20Object%20Reference) (OtherBodyIndex :type Integer) (bFromSweep :type Boolean) (SweepResult :type Hit%20Result%20Structure%20%28by%20ref%29))
  (bind _returnvalue (Actor|GetComponentbyClass OtherActor "/Game/OpenWorldLocomotion/CharacterComponents/SystemComponents/OWL_Climbing_BP.OWL_Climbing_BP_C"))
  (Utilities|IsValid _returnvalue
    (:Is%20Valid
      (Default|SetClimbonMovingObjects _returnvalue true))))

(event OnComponentBeginOverlap(Box)
  (params (OverlappedComponent :type Primitive%20Component%20Object%20Reference) (OtherActor :type Actor%20Object%20Reference) (OtherComp :type Primitive%20Component%20Object%20Reference) (OtherBodyIndex :type Integer) (bFromSweep :type Boolean) (SweepResult :type Hit%20Result%20Structure%20%28by%20ref%29))
  (bind _returnvalue (Transformation|GetActorLocation))
  (bind _points (Variables|Default|GetPoints))
  (if (not (Variables|Default|GetStart))
    (Utilities|Casting|CastToCharacter OtherActor)
    (Variables|/Script/Engine.PrimitiveComponent|SetbGenerateOverlapEvents (Variables|Default|GetBox) false)
    (Variables|Default|SetStart true)
    (Utilities|FlowControl|Delay 0.3)
    (if (Variables|Default|GetReturn)
      (Utilities|Array|Insert _points _returnvalue)
      (Variables|Default|SetIndex 1)
      (else
        (Utilities|Array|Add _points _returnvalue)))
    (Components|MoveComponentTo (Variables|Default|GetStaticMesh) (Utilities|Array|Get(acopy) (Variables|Default|GetPoints) (Variables|Default|GetIndex)) "0, 0, 0" false false (/ (Math|Vector|Distance(Vector) (Utilities|Array|Get(acopy) (Variables|Default|GetPoints) (Variables|Default|GetIndex)) (Transformation|GetActorLocation)) (Variables|Default|GetVelocity)) false :!label _label)
    (Utilities|FlowControl|Delay (Variables|Default|GetDelay))
    (Utilities|FlowControl|Sequence
      (:then_0
        (if (Variables|Default|GetReturn)
          (if (Variables|Default|GetReturning)
            (if (<= (Variables|Default|GetIndex) 0)
              (Variables|Default|SetReturning false)
              (Variables|Default|SetIndex 1)
              (else
                (Math|Integer|DecrementInt (Variables|Default|GetIndex))))
            (elif (>= (Variables|Default|GetIndex) (Utilities|Array|LastIndex (Variables|Default|GetPoints)))
              (Variables|Default|SetReturning true)
              (Math|Integer|DecrementInt (Variables|Default|GetIndex))
              (else
                (Math|Integer|IncrementInt (Variables|Default|GetIndex)))))
          (elif (>= (Variables|Default|GetIndex) (Utilities|Array|LastIndex (Variables|Default|GetPoints)))
            (Variables|Default|SetIndex 0)
            (else
              (Math|Integer|IncrementInt (Variables|Default|GetIndex))))))
      (:then_1
        (goto _label)))))

(event OnComponentEndOverlap(ClimbOnMovingObjectsTrigger)
  (params (OverlappedComponent :type Primitive%20Component%20Object%20Reference) (OtherActor :type Actor%20Object%20Reference) (OtherComp :type Primitive%20Component%20Object%20Reference) (OtherBodyIndex :type Integer))
  (bind _returnvalue (Actor|GetComponentbyClass OtherActor "/Game/OpenWorldLocomotion/CharacterComponents/SystemComponents/OWL_Climbing_BP.OWL_Climbing_BP_C"))
  (Utilities|IsValid _returnvalue
    (:Is%20Valid
      (Default|SetClimbonMovingObjects _returnvalue false))))

(fn ConstructionScript)