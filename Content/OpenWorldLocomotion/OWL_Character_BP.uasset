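; Example Open World Locomotion player character that layers weapons, stamina, cameras, HUD prompts and object grabbing over the OWL components.
; Overlay changes spawn or destroy weapons, whose aim target comes from a camera trace and feeds hand IK.
; Climbing, gliding, swimming and sprinting drive stamina, which disables those abilities or swim input when empty.
; Timelines serve as on-demand ticks for aiming, IK and stamina, while Tick updates sprint camera and prompts.
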(event Custom|Grabbing%20Info%20Timer
  (params (bLooping :type Boolean))
  (Utilities|Time|SetTimerbyEvent (delegate Custom|GrabbingInfo) 0.01 bLooping))

(event Custom|GrabbingInfo
  (bind _originaldistancetoobject (Variables|Default|GetOriginalDistanceToObject))
  (bind _fpc (Variables|Default|GetFPC))
  (bind _returnvalue (Math|Vector|GetForwardVector _fpc))
  (bind _returnvalue_2 (Transformation|GetWorldLocation _fpc))
  (bind _returnvalue_3 (* _returnvalue _originaldistancetoobject))
  (bind _returnvalue_4 (+ _returnvalue_2 _returnvalue_3))
  (if (Variables|Default|GetGrabMode)
    (if (not (Physics|IsSimulatingPhysics (Variables|Default|GetGrabbedComponent) "None"))
      (Physics|Components|PhysicsHandle|SetTargetLocation (Variables|Default|GetPhysicsHandle) _returnvalue_4)
      (Transformation|SetWorldLocation (Variables|Default|GetGrabbedComponent) _returnvalue_4 true false))
    (else
      (Utilities|FlowControl|Delay 0.2)
      (Variables|Default|SetGrabbedSomething? false))))

(event Custom|OnSprintingChanged_Event
  (params (Sprinting :type Boolean))
  ;[1 1 1] Stamina System (example)
  ;;[1 1 1] Event Dispatchers (bound on Event Begin Play)
  (if Sprinting
    (if (not (Variables|Stamina|GetDisable%20Stamina))
      (Variables|Stamina|Variables|SetUseStamina true)
      (Audio|Components|Audio|Play (Variables|Default|GetStamina_Timeline)))
    (elif (not (Utilities|Array|ContainsItem (Utilities|Array|MakeArray "NewEnumerator3" "NewEnumerator4" "NewEnumerator7") (Variables|/Game/OpenWorldLocomotion/CharacterComponents/OWL_BaseComponent_BP.OWL_BaseComponent_BP_C|GetLocomotionState (Variables|Default|GetOWL_BaseComponent_BP))))
      (Variables|Stamina|Variables|SetUseStamina false))))

(event Custom|ChangeLocomotionState_Event
  (params (NewLocomotionState :type E_LocomotionStates%20Enum :default "NewEnumerator0") (PrevLocomotionState :type E_LocomotionStates%20Enum :default "NewEnumerator0"))
  ;[1 1 1] Stamina System (example)
  ;;[1 1 1] Event Dispatchers (bound on Event Begin Play)
  (if (Utilities|Array|ContainsItem (Utilities|Array|MakeArray "NewEnumerator3" "NewEnumerator4" "NewEnumerator7") NewLocomotionState)
    (if (not (Variables|Stamina|GetDisable%20Stamina))
      (Variables|Stamina|Variables|SetUseStamina true)
      (Audio|Components|Audio|Play (Variables|Default|GetStamina_Timeline)))
    (elif (not (Variables|/Game/OpenWorldLocomotion/CharacterComponents/OWL_BaseComponent_BP.OWL_BaseComponent_BP_C|GetIsSprinting (Variables|Default|GetOWL_BaseComponent_BP)))
      (Variables|Stamina|Variables|SetUseStamina false))))

(event Custom|DisableStamina_SERVER
  (params (DisableStamina :type Boolean))
  ;[1 1 1] Stamina System (example)
  ;;[1 1 1] Disable Stamina
  (Variables|Stamina|SetDisable%20Stamina DisableStamina))

(event Custom|SwitchWeapon
  ;[1 0 1] Switch weapon (example)
  (bind _output_get (Variables|Variables|SetCurrentOverlay (Utilities|Array|Get(acopy) (Variables|Default|GetWeapons) (Math|Integer|SelectInt (+ (Utilities|Array|FindItem (Variables|Default|GetWeapons) (Variables|Variables|GetCurrentOverlay)) 1) 0 (Utilities|Array|IsValidIndex (Variables|Default|GetWeapons) (+ (Utilities|Array|FindItem (Variables|Default|GetWeapons) (Variables|Variables|GetCurrentOverlay)) 1))))))
  (CallFunction|BPISwitchOverlay _output_get))

(event Custom|ClimbingJump_Event
  ;[1 1 1] Stamina System (example)
  ;;[1 1 1] Event Dispatchers (bound on Event Begin Play)
  (if (not (Variables|Stamina|GetDisable%20Stamina))
    (Variables|Stamina|Variables|SetStamina (- (Variables|Stamina|Variables|GetStamina) 2e+01))))

(event EventDestroyed
  ;[1 0 1] Spawning a weapon (example)
  (|CallParentFunction)
  (bind _currentweapon (Variables|Variables|GetCurrentWeapon)
    (:then
      (Actor|DestroyActor _currentweapon))
    (:else)))

(event EventBPIonOverlayEnabled
  (params (Enable :type Boolean))
  ;[1 0 1] Spawning a weapon (example)
  (|CallParentFunction Enable)
  (|Spawn/DespawnWeapon_Graph Enable))

(event EventBPIIsAiming
  (params (Aiming :type Boolean))
  ;[1 0 1] Aim weapon (example)
  (if Aiming
    (Components|Timeline|PlayfromStart (Variables|Default|GetAimingTrace_Timeline))
    (CallFunction|BPIModifyMovementSpeed true 1.5e+02 true)
    (else
      (Audio|Components|Audio|Stop (Variables|Default|GetAimingTrace_Timeline))
      (CallFunction|BPIModifyMovementSpeed false 0.0 false))))

(event EventTick
  (params (DeltaSeconds :type Float%20%28single-precision%29))
  ;[1 1 1] Tick event
  (|CallParentFunction DeltaSeconds)
  (Utilities|SprintCamera) ; Moves third person camera back when sprinting
  ;;[1 1 1] Screen Prompts (HUD)
  (|ManualClimbingScreenPrompt)
  (|VaultingScreenPrompt))

(event EventBeginPlay
  ;[1 1 1] Begin Play event
  (|CallParentFunction)
  (bind _foundwidgets (Widget|GetAllWidgetsOfClass "/Game/OpenWorldLocomotion/HUD/HUD_Widget.HUD_Widget_C" true))
  (Variables|HUD|SetHUD (Utilities|Array|Get(acopy) _foundwidgets))
  (CallFunction|SwitchWeapon)
  (EventDispatchers|AssignClimbingJump (Variables|Default|GetOWL_Climbing_BP) (EventDispatchers|CreateEvent :!event Custom|ClimbingJump_Event))
  (EventDispatchers|BindEventtoOnSprintingChanged (Variables|Default|GetOWL_BaseComponent_BP) (EventDispatchers|CreateEvent :!event Custom|OnSprintingChanged_Event))
  (EventDispatchers|BindEventtoChangeLocomotionState (Variables|Default|GetOWL_BaseComponent_BP) (EventDispatchers|CreateEvent :!event Custom|ChangeLocomotionState_Event)))

(event Input|ActionEvents|InputActionMenu
  (params (Key :type Key%20Structure :default "None"))
  ;[1 1 1] HUD
  (:Pressed
    (bind _menu (Variables|HUD|GetMenu)
      (:then
        (Widget|RemovefromParent _menu)
        (Variables|HUD|SetMenu 0)
        (Variables|/Script/Engine.PlayerController|SetbShowMouseCursor (Game|GetPlayerController 0) false)
        (Game|SetGamePaused false))
      (:else
        (bind _returnvalue (UserInterface|CreateWidget "/Game/OpenWorldLocomotion/HUD/Menu_Widget.Menu_Widget_C"))
        (bind _output_get (Variables|HUD|SetMenu _returnvalue))
        (UserInterface|Viewport|AddtoViewport _output_get 0)
        (Variables|/Script/Engine.PlayerController|SetbShowMouseCursor (Game|GetPlayerController 0) true)
        (Game|SetGamePaused true)))))

(event Input|ActionEvents|InputActionChangeCamera
  (params (Key :type Key%20Structure :default "None"))
  ;[1 1 1] ChangeCamera
  (:Pressed
    (switch Utilities|FlowControl|Switch|SwitchonE_CameraType (Variables|/Game/OpenWorldLocomotion/CharacterComponents/OWL_BaseComponent_BP.OWL_BaseComponent_BP_C|GetCameraType (Variables|Default|GetOWL_BaseComponent_BP))
      (:NewEnumerator0
        (Components|Activation|Deactivate (Variables|Default|GetFPC))
        (Components|Activation|Activate (Variables|Default|GetTPC) true))
      (:NewEnumerator1
        (Components|Activation|Deactivate (Variables|Default|GetTPC))
        (Components|Activation|Activate (Variables|Default|GetFPC) true)))))

(event Input|MouseEvents|MouseWheelAxis
  (params (AxisValue :type Float%20%28single-precision%29))
  (bind _returnvalue (* AxisValue 1e+01))
  (if (Variables|Default|GetGrabMode)
    (if (Variables|Default|GetRoationModeVerticle)
      (Transformation|AddWorldRotation (Variables|Default|GetGrabbedComponent) (Math|Rotator|MakeRotator 0.0 0.0 _returnvalue) false false)
      (else
        (Transformation|AddWorldRotation (Variables|Default|GetGrabbedComponent) (Math|Rotator|MakeRotator 0.0 _returnvalue 0.0) false false)))))

(event Input|MouseEvents|LeftMouseButton
  (params (Key :type Key%20Structure :default "None"))
  (bind _fpc (Variables|Default|GetFPC))
  (bind _returnvalue (Transformation|GetWorldLocation _fpc))
  (:Pressed
    (Variables|Default|SetGrabMode true)
    (if (Variables|Default|GetGrabMode)
      (CallFunction|GrabbingInfoTimer true)
      (bind (_outhit _returnvalue_2) (Collision|LineTraceByChannel _returnvalue (+ _returnvalue (* (Math|Vector|GetForwardVector _fpc) (Math|Float|MakeLiteralFloat 5e+02))) "TraceTypeQuery1" true 0 "Persistent"))
      (if _returnvalue_2
        (if (== (Variables|/Script/Engine.SceneComponent|GetMobility (.HitComponent (Collision|BreakHitResult _outhit))) (Utilities|Enum|LiteralenumEComponentMobility "Movable"))
          (Variables|Default|SetOriginalDistanceToObject (.Distance (Collision|BreakHitResult _outhit)))
          (bind _output_get (Variables|Default|SetGrabbedComponent (.HitComponent (Collision|BreakHitResult _outhit))))
          (Physics|SetSimulatePhysics _output_get false)
          (if (Physics|IsSimulatingPhysics _output_get "None")
            (Class|PhysicsHandleComponent|GrabComponentatLocation (Variables|Default|GetPhysicsHandle) (Variables|Default|GetGrabbedComponent) "None" (.Location (Collision|BreakHitResult _outhit))))))))
  (:Released
    (Variables|Default|SetGrabMode false)
    (CallFunction|GrabbingInfoTimer false)
    (if (not (Variables|Default|GetGrabMode))
      (Physics|SetSimulatePhysics (Variables|Default|GetGrabbedComponent) true)
      (Variables|Default|SetGrabbedComponent 0)
      (Physics|Components|PhysicsHandle|ReleaseComponent (Variables|Default|GetPhysicsHandle)))))

(event Input|MouseEvents|RightMouseButton
  (params (Key :type Key%20Structure :default "None"))
  (:Pressed
    (Variables|Default|SetRoationModeVerticle (not (Variables|Default|GetRoationModeVerticle)))))

(event Input|KeyboardEvents|Tab
  (params (Key :type Key%20Structure :default "None"))
  ;[1 0 1] Switch weapon (example)
  (:Pressed
    (CallFunction|SwitchWeapon)))

(event Input|KeyboardEvents|1
  (params (Key :type Key%20Structure :default "None"))
  ;[1 1 1] Stamina System (example)
  ;;[1 1 1] Disable Stamina
  (:Pressed
    (bind _output_get (Variables|Stamina|SetDisable%20Stamina (not (Variables|Stamina|GetDisable%20Stamina))))
    (Networking|SwitchHasAuthority
      (:Remote
        (CallFunction|DisableStaminaSERVER _output_get)))))

(fn ConstructionScript
  (|CallParentFunction))

(fn StaminaSystem
  (bind _owl_basecomponent_bp (Variables|Default|GetOWL_BaseComponent_BP))
  (bind _owl_basecomponent_bp_2 (Variables|Default|GetOWL_BaseComponent_BP))
  (bind _staminaregen (Variables|Stamina|GetStaminaRegen))
  (bind _locomotionstate (Variables|/Game/OpenWorldLocomotion/CharacterComponents/OWL_BaseComponent_BP.OWL_BaseComponent_BP_C|GetLocomotionState _owl_basecomponent_bp))
  (bind _locomotionstate_2 (Variables|/Game/OpenWorldLocomotion/CharacterComponents/OWL_BaseComponent_BP.OWL_BaseComponent_BP_C|GetLocomotionState _owl_basecomponent_bp_2))
  (bind (_value _returnvalue) (Utilities|Map|Find _staminaregen _locomotionstate))
  (Utilities|FlowControl|Sequence
    (:then_0
      ;[1 1 1] Drain stamina conditions
      (Variables|Stamina|Variables|SetDrainStamina (and (or (Utilities|Enum|Equal(Enum) _locomotionstate_2 "NewEnumerator4") (and (Math|Boolean|ORBoolean (Utilities|Enum|Equal(Enum) _locomotionstate_2 "NewEnumerator3") (Utilities|Enum|Equal(Enum) _locomotionstate_2 "NewEnumerator7") (Variables|/Game/OpenWorldLocomotion/CharacterComponents/OWL_BaseComponent_BP.OWL_BaseComponent_BP_C|GetIsSprinting (Variables|Default|GetOWL_BaseComponent_BP))) (not (Math|Vector|VectorIsNearlyZero (Transformation|GetVelocity) 5.0)))) (not (Variables|Stamina|GetDisable%20Stamina)))))
    (:then_1
      ;[1 1 1] Change stamina value
      (if (Variables|Stamina|Variables|GetDrainStamina)
        (Variables|Stamina|Variables|SetStamina (Math|Float|Clamp(Float) (- (Variables|Stamina|Variables|GetStamina) (* (Variables|Stamina|GetStamina%20Drain) (Utilities|Time|GetWorldDeltaSeconds))) 0.0 (Variables|Stamina|GetMaxStamina)))
        (elif (not (== (Variables|Stamina|Variables|GetStamina) (Variables|Stamina|GetMaxStamina)))
          (Variables|Stamina|Variables|SetStamina (Math|Float|Clamp(Float) (+ (Variables|Stamina|Variables|GetStamina) (* (Math|Float|SelectFloat _value (.Value (Utilities|Map|Find (Variables|Stamina|GetStaminaRegen) "NewEnumerator1")) _returnvalue) (Utilities|Time|GetWorldDeltaSeconds))) 0.0 (Variables|Stamina|GetMaxStamina))))))
    (:then_2
      ;[1 1 1] If stamina reaches 0, disable Climbing Gliding and Sprinting, reenable them when it regenereates above the threshold
      (if (<= (Variables|Stamina|Variables|GetStamina) 0.0)
        (CallFunction|StaminaLost)
        (elif (and (> (Variables|Stamina|Variables|GetStamina) (Variables|Stamina|GetStaminaThreshold)) (Variables|Stamina|Variables|GetNoStamina))
          (CallFunction|StaminaRegained))))
    (:then_3
      ;[1 1 1] Stops the timeline when the stamina is full and Use Stamina is false
      (if (and (not (Variables|Stamina|Variables|GetUseStamina)) (== (Variables|Stamina|Variables|GetStamina) (Variables|Stamina|GetMaxStamina)))
        (Audio|Components|Audio|Stop (Variables|Default|GetStamina_Timeline))
        (return)))))

(fn StaminaLost
  (bind _returnvalue (Pawn|GetController))
  (bind _owl_basecomponent_bp (Variables|Default|GetOWL_BaseComponent_BP))
  (if (not (Variables|Stamina|Variables|GetNoStamina))
    (if (not (Variables|/Game/OpenWorldLocomotion/CharacterComponents/SystemComponents/OWL_Climbing_BP.OWL_Climbing_BP_C|GetJumpClimb (Variables|Default|GetOWL_Climbing_BP)))
      (Variables|Stamina|Variables|SetNoStamina true)
      (Utilities|FlowControl|Sequence
        (:then_0
          (Variables|/Game/OpenWorldLocomotion/CharacterComponents/OWL_BaseComponent_BP.OWL_BaseComponent_BP_C|SetDisableSprinting _owl_basecomponent_bp true)
          (if (Variables|/Game/OpenWorldLocomotion/CharacterComponents/OWL_BaseComponent_BP.OWL_BaseComponent_BP_C|GetCanSprint _owl_basecomponent_bp)
            (Default|Sprint (Variables|Default|GetOWL_BaseComponent_BP) false)))
        (:then_1
          (Default|CallDisableGlidingOverride (Variables|Default|GetOWL_BaseComponent_BP) true true self)
          (Default|CallDisableClimbingOverride (Variables|Default|GetOWL_BaseComponent_BP) true false true self)
          (switch Utilities|FlowControl|Switch|SwitchonE_LocomotionStates (Variables|/Game/OpenWorldLocomotion/CharacterComponents/OWL_BaseComponent_BP.OWL_BaseComponent_BP_C|GetLocomotionState (Variables|Default|GetOWL_BaseComponent_BP))
            (:NewEnumerator7
              (Utilities|IsValid _returnvalue
                (:Is%20Valid
                  (Input|SetIgnoreMoveInput _returnvalue true)
                  (Variables|Stamina|Variables|SetStamina_IsInputIgnored true))))))))))

(fn StaminaRegained
  (bind _returnvalue (Pawn|GetController))
  (if (Variables|Stamina|Variables|GetNoStamina)
    (Variables|Stamina|Variables|SetNoStamina false)
    (Utilities|FlowControl|Sequence
      (:then_0
        (Variables|/Game/OpenWorldLocomotion/CharacterComponents/OWL_BaseComponent_BP.OWL_BaseComponent_BP_C|SetDisableSprinting (Variables|Default|GetOWL_BaseComponent_BP) false))
      (:then_1
        (Default|CallDisableGlidingOverride (Variables|Default|GetOWL_BaseComponent_BP) false true self)
        (Default|CallDisableClimbingOverride (Variables|Default|GetOWL_BaseComponent_BP) false false true self)
        (Utilities|IsValid _returnvalue
          (:Is%20Valid
            (if (Variables|Stamina|Variables|GetStamina_IsInputIgnored)
              (Input|SetIgnoreMoveInput _returnvalue false))))))))