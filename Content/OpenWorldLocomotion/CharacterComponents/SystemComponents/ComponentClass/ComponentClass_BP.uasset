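; ComponentClass_BP is a component Blueprint in the OpenWorldLocomotion system components, apparently a shared base, that sets up references on its owning Character.
; On BeginPlay it caches the Character, its OWL_BaseComponent_BP and CharacterMovement.
; Tick prerequisites make it tick after the base component and make the Character tick after it.
; It prints a message if the owner is not a Character or lacks the base component.
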(event EventBeginPlay
  (bind _ascharacter (Utilities|Casting|CastToCharacter (Components|GetOwner))
    (:then
      (bind _output_get (Variables|DoNotModify|SetCharacter _ascharacter))
      (Utilities|IsValid (Actor|GetComponentbyClass _output_get "/Game/OpenWorldLocomotion/CharacterComponents/OWL_BaseComponent_BP.OWL_BaseComponent_BP_C")
        (:Is%20Valid
          (bind _output_get_2 (Variables|DoNotModify|SetBaseComponent (Actor|GetComponentbyClass _output_get "/Game/OpenWorldLocomotion/CharacterComponents/OWL_BaseComponent_BP.OWL_BaseComponent_BP_C")))
          (Class|ActorComponent|AddTickPrerequisiteComponent _output_get_2) ; Makes this component tick after the BaseComponent
          (Class|Actor|AddTickPrerequisiteComponent (Variables|DoNotModify|GetCharacter) self) ; Makes the character tick after the component
          (Variables|DoNotModify|SetCharacterMovement (Variables|/Script/Engine.Character|GetCharacterMovement (Variables|DoNotModify|GetCharacter))))
        (:Is%20Not%20Valid
          (Development|PrintString "Base Component not found. Please add OWL_BaseComponent_BP to your character blueprint"))))
    (:CastFailed
      (Development|PrintString "This actor is not a Character class. Add this component only to the Character class blueprints."))))