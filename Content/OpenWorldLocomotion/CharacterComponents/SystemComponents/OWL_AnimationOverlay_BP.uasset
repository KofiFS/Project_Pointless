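; Character component that manages animation overlays with pull-out and put-away montages, aiming and combat stance, driven by an OverlayData asset.
; Server RPCs and OnRep handlers sync state, notifying the character and base locomotion component and optionally restricting climbing or gliding.
; Locomotion state changes and optional sliding checks toggle the overlay.
; Tick also updates hip rotation and drops combat stance after a retriggerable delay.
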(event EventBeginPlay
  ;[1 0 1] Initialize component
  (|CallParentFunction)
  (Initialization|Initialize))

(event Custom|OverlayEnabled_SERVER
  (params (Enabled :type Boolean))
  ;[1 1 1] OverlayEnabled
  (Variables|OverlayVariables|SetOverlayEnabled Enabled))

(event Custom|Aiming_SERVER
  (params (Aiming :type Boolean))
  ;[1 1 1] Aiming
  (Variables|OverlayVariables|SetAiming Aiming))

(event Custom|SwitchOverlay_SERVER
  (params (OverlayData :type Anim%20Overlay%20PDA%20Object%20Reference))
  ;[1 1 1] SwitchOverlay
  (Variables|OverlayVariables|SetOverlayData OverlayData))

(event Custom|ActivateOverlay_MULTICAST
  (params (CanActivateOverlay :type Boolean))
  ;[1 1 1] ActivateOverlay
  (if (not (Pawn|IsLocallyControlled (Variables|Default|GetCharacter)))
    (CallFunction|ActivateOverlayEvent CanActivateOverlay)))

(event Custom|ActivateOverlay_SERVER
  (params (CanActivateOverlay :type Boolean))
  ;[1 1 1] ActivateOverlay
  (CallFunction|ActivateOverlayMULTICAST CanActivateOverlay))

(event EventTick
  (params (DeltaSeconds :type Float%20%28single-precision%29))
  (|CallParentFunction DeltaSeconds)
  (Base|SetHipRotation)
  (|DisableCombatStance)
  (|DisableOverlayWhenSliding_))

(fn SwitchOverlay
  (params (OverlayData :type Anim%20Overlay%20PDA%20Object%20Reference))
  (if (!= OverlayData (Variables|OverlayVariables|GetOverlayData))
    (bind _output_get (Variables|OverlayVariables|SetOverlayData OverlayData))
    (if (not (Ability|HasAuthority (Variables|Default|GetCharacter)))
      (CallFunction|SwitchOverlaySERVER _output_get))))

(fn Aim
  (params (Aim :type Boolean))
  (if (Variables|OverlayVariables|GetOverlayEnabled)
    (bind _overlaydata (Variables|OverlayVariables|GetOverlayData)
      (:then
        (if (Variables|/Game/OpenWorldLocomotion/Data/DataAsset/AnimOverlay_PDA.AnimOverlay_PDA_C|GetCanBeAimed _overlaydata)
          (Variables|OverlayVariables|SetAiming Aim)
          (Utilities|FlowControl|Sequence :!label _label
            (:then_0
              ;[1 1 1] Disables climbing or/and gliding while aiming (controled through variables)
              (if (or (Variables|Overlay|Aiming|GetAiming_DisableClimbing) (Variables|Overlay||Aiming|GetAiming_VaultOnly))
                (Default|CallDisableClimbingOverride (Variables|Default|GetBaseComponent) (or (and (Variables|OverlayVariables|GetOverlayEnabled) (Variables|Overlay|OverlayEnabled|GetOverlayEnabled_DisableClimbing)) (and (Variables|OverlayVariables|GetAiming) (Variables|Overlay|Aiming|GetAiming_DisableClimbing))) (or (and (Variables|OverlayVariables|GetOverlayEnabled) (Variables|Overlay||OverlayEnabled|GetOverlayEnabled_VaultOnly)) (and (Variables|OverlayVariables|GetAiming) (Variables|Overlay||Aiming|GetAiming_VaultOnly))) true self))
              (if (Variables|Overlay|Aiming|GetAiming_DisableGliding)
                (Default|CallDisableGlidingOverride (Variables|Default|GetBaseComponent) (or (Variables|OverlayVariables|GetAiming) (and (Variables|OverlayVariables|GetOverlayEnabled) (Variables|Overlay|OverlayEnabled|GetOverlayEnabled_DisableGliding))) true self)))
            (:then_1
              (if (not (Ability|HasAuthority (Variables|Default|GetCharacter)))
                (CallFunction|AimingSERVER (Variables|OverlayVariables|GetAiming)))))
          (else
            (if (Variables|OverlayVariables|GetAiming) :!label _label_2
              (Variables|OverlayVariables|SetAiming false)
              (goto _label)))))
      (:else
        (goto _label_2)))
    (else
      (goto _label_2))))

(fn ActivateOverlay
  (params (CanActivateOverlay :type Boolean))
  (CallFunction|ActivateOverlayEvent CanActivateOverlay)
  (if (not (Class|KismetSystemLibrary|IsStandalone))
    (CallFunction|ActivateOverlaySERVER CanActivateOverlay)))

(fn SetHipRotation
  (bind _basecomponent (Variables|Default|GetBaseComponent))
  (bind _overlaydata (Variables|OverlayVariables|GetOverlayData))
  (if (and (Variables|OverlayVariables|GetOverlayEnabled) (Utilities|IsValid _overlaydata))
    (Variables|/Game/OpenWorldLocomotion/CharacterComponents/OWL_BaseComponent_BP.OWL_BaseComponent_BP_C|SetHipRotation _basecomponent (select (Variables|/Game/OpenWorldLocomotion/CharacterComponents/OWL_BaseComponent_BP.OWL_BaseComponent_BP_C|GetCombatStance (Variables|Default|GetBaseComponent)) (Variables|/Game/OpenWorldLocomotion/Data/DataAsset/AnimOverlay_PDA.AnimOverlay_PDA_C|GetHipRotation_Combat _overlaydata) (Variables|/Game/OpenWorldLocomotion/Data/DataAsset/AnimOverlay_PDA.AnimOverlay_PDA_C|GetHipRotation_Relaxed _overlaydata)))
    (else
      (Variables|/Game/OpenWorldLocomotion/CharacterComponents/OWL_BaseComponent_BP.OWL_BaseComponent_BP_C|SetHipRotation _basecomponent "NewEnumerator0"))))

(fn OnRepOverlayEnabled
  (Class|OWLInterfaceBPI|BPIonOverlayEnabled(Message) (Variables|Default|GetCharacter) (Variables|OverlayVariables|GetOverlayEnabled))
  (Utilities|FlowControl|Sequence
    (:then_0
      (if (Variables|OverlayVariables|GetOverlayEnabled)
        (bind _overlaydata (Variables|OverlayVariables|GetOverlayData)
          (:then
            (Overlay|SetCombatStance (Variables|/Game/OpenWorldLocomotion/Data/DataAsset/AnimOverlay_PDA.AnimOverlay_PDA_C|GetCombatStanceOnOverlayEnabled _overlaydata)))
          (:else))))
    (:then_1
      (Utilities|FlowControl|Sequence
        (:then_0
          ;[1 1 1] Disables climbing or/and gliding when overlay is enabled (controled through variables)
          (if (or (Variables|Overlay|OverlayEnabled|GetOverlayEnabled_DisableClimbing) (Variables|Overlay||OverlayEnabled|GetOverlayEnabled_VaultOnly))
            (Default|CallDisableClimbingOverride (Variables|Default|GetBaseComponent) (and (Variables|OverlayVariables|GetOverlayEnabled) (Variables|Overlay|OverlayEnabled|GetOverlayEnabled_DisableClimbing)) (and (Variables|OverlayVariables|GetOverlayEnabled) (Variables|Overlay||OverlayEnabled|GetOverlayEnabled_VaultOnly)) true self)))
        (:then_1
          (if (Variables|Overlay|OverlayEnabled|GetOverlayEnabled_DisableGliding)
            (Default|CallDisableGlidingOverride (Variables|Default|GetBaseComponent) (Variables|OverlayVariables|GetOverlayEnabled) true self)))))))

(fn OnRepOverlayData
  (Utilities|IsValid (Variables|OverlayVariables|GetOverlayData)
    (:Is%20Valid
      (Variables|OverlayVariables|SetDisableCombatStanceDelay (Variables|/Game/OpenWorldLocomotion/Data/DataAsset/AnimOverlay_PDA.AnimOverlay_PDA_C|GetDisableCombatStanceDelay (Variables|OverlayVariables|GetOverlayData)))
      (Variables|OverlayVariables|SetDisableCombatStanceOnlyWhenStatic (Variables|/Game/OpenWorldLocomotion/Data/DataAsset/AnimOverlay_PDA.AnimOverlay_PDA_C|GetDisableCombatStanceOnlyWhenStatic (Variables|OverlayVariables|GetOverlayData)))
      (if (Variables|OverlayVariables|GetOverlayEnabled)
        (Class|OWLInterfaceBPI|BPIonOverlayEnabled(Message) (Variables|Default|GetCharacter) (Variables|OverlayVariables|GetOverlayEnabled))
        (Overlay|SetCombatStance (Variables|/Game/OpenWorldLocomotion/Data/DataAsset/AnimOverlay_PDA.AnimOverlay_PDA_C|GetCombatStanceOnOverlayEnabled (Variables|OverlayVariables|GetOverlayData)))
        (if (and (Variables|Overlay|GetPlayMontagesWhenSwitchingOverlays) (Variables|OverlayVariables|GetCanActivateOverlay))
          (Animation|Montage|MontagePlay (Components|SkeletalMesh|GetAnimInstance (Variables|/Script/Engine.Character|GetMesh (Variables|Default|GetCharacter))) (Overlay|FindAnimMontage (Variables|/Game/OpenWorldLocomotion/Data/DataAsset/AnimOverlay_PDA.AnimOverlay_PDA_C|GetPullOutAnim (Variables|OverlayVariables|GetOverlayData))) (Variables|Overlay|GetMontagesPlayRate) "Duration" 0.0 true))))
    (:Is%20Not%20Valid
      (Variables|OverlayVariables|SetOverlayEnabled false)
      (Overlay|SetCombatStance false)
      (Variables|OverlayVariables|SetCanActivateOverlay false)
      (Variables|OverlayVariables|SetAiming false))))

(fn OnRepAiming
  (Utilities|FlowControl|Sequence
    (:then_0
      (if (Variables|OverlayVariables|GetAiming)
        (Overlay|SetCombatStance true)
        (Default|SwitchRotationMode (Variables|Default|GetBaseComponent) "NewEnumerator1")))
    (:then_1
      (Variables|/Game/OpenWorldLocomotion/CharacterComponents/OWL_BaseComponent_BP.OWL_BaseComponent_BP_C|SetLockRotationMode (Variables|Default|GetBaseComponent) (Variables|OverlayVariables|GetAiming))
      (Class|OWLInterfaceBPI|BPIIsAiming(Message) (Variables|Default|GetCharacter) (Variables|OverlayVariables|GetAiming))
      (Default|CallOnAimingChange (Variables|Default|GetBaseComponent) (Variables|OverlayVariables|GetAiming)))))

(fn SetCombatStance
  (params (CombatStance :type Boolean))
  (bind _output_get (Variables|/Game/OpenWorldLocomotion/CharacterComponents/OWL_BaseComponent_BP.OWL_BaseComponent_BP_C|SetCombatStance (Variables|Default|GetBaseComponent) CombatStance))
  (Default|CallOnStanceChanged (Variables|Default|GetBaseComponent) _output_get))

(fn InputActivateOverlay
  (bind _canactivateoverlay (Variables|OverlayVariables|GetCanActivateOverlay))
  (bind _returnvalue (not _canactivateoverlay))
  (if (Utilities|Array|ContainsItem (Variables|Overlay|GetCanActivateOverlayStates) (Variables|/Game/OpenWorldLocomotion/CharacterComponents/OWL_BaseComponent_BP.OWL_BaseComponent_BP_C|GetLocomotionState (Variables|Default|GetBaseComponent)))
    (if (Class|KismetSystemLibrary|IsStandalone)
      _
      (else
        (CallFunction|ActivateOverlaySERVER _returnvalue)))
    (CallFunction|ActivateOverlayEvent _returnvalue)))

(fn FindAnimMontage
  (params (InputPin :type Map%20of%20Character%20Class%20References%20to%20Objects))
  (bind _character (Variables|Default|GetCharacter))
  (bind _returnvalue (Utilities|GetClass _character))
  (bind (_value _returnvalue_2) (Utilities|Map|Find InputPin _returnvalue))
  (if _returnvalue_2
    (return _value)
    (else
      (bind _keys (Utilities|Map|Keys InputPin))
      (for _array_element _keys
        (if (Utilities|ClassIsChildOf _returnvalue _array_element)
          (return (.Value (Utilities|Map|Find InputPin _array_element)))))
      (return 0))))

(fn SetHandIK
  (params (EnableLeftHandIK :type Boolean) (LeftHandIK :type Hand%20IK%20Struct%20Structure) (EnableRightHandIK :type Boolean) (RightHandIK :type Hand%20IK%20Struct%20Structure))
  (Variables|HandIK|SetEnableLeftHandIK EnableLeftHandIK)
  (Variables|HandIK|SetLeftHandIK LeftHandIK)
  (Variables|HandIK|SetEnableRightHandIK EnableRightHandIK)
  (Variables|HandIK|SetRightHandIK RightHandIK))

(event Custom|ActivateOverlay_Event
  (params (CanActivateOverlay :type Boolean))
  (bind _overlaydata (Variables|OverlayVariables|GetOverlayData))
  (Variables|OverlayVariables|GetOverlayData
    (:then
      (Variables|OverlayVariables|SetCanActivateOverlay CanActivateOverlay)
      (if (Utilities|Array|ContainsItem (Variables|Overlay|GetOverlayEnabledForLocomotionState) (Variables|/Game/OpenWorldLocomotion/CharacterComponents/OWL_BaseComponent_BP.OWL_BaseComponent_BP_C|GetLocomotionState (Variables|Default|GetBaseComponent)))
        (bind _returnvalue (Animation|Montage|MontagePlay (Components|SkeletalMesh|GetAnimInstance (Variables|/Script/Engine.Character|GetMesh (Variables|Default|GetCharacter))) (select (Variables|OverlayVariables|GetCanActivateOverlay) (Overlay|FindAnimMontage (Variables|/Game/OpenWorldLocomotion/Data/DataAsset/AnimOverlay_PDA.AnimOverlay_PDA_C|GetPullOutAnim _overlaydata)) (Overlay|FindAnimMontage (Variables|/Game/OpenWorldLocomotion/Data/DataAsset/AnimOverlay_PDA.AnimOverlay_PDA_C|GetPutAwayAnim _overlaydata))) (Variables|Overlay|GetMontagesPlayRate) "Duration" 0.0 true))
        (if (Variables|OverlayVariables|GetCanActivateOverlay)
          (Variables|OverlayVariables|SetOverlayEnabled true)
          (else
            (Variables|OverlayVariables|SetAiming false)
            (Overlay|SetCombatStance false)
            (Utilities|FlowControl|RetriggerableDelay _returnvalue)
            (if (not (Variables|OverlayVariables|GetCanActivateOverlay))
              (Variables|OverlayVariables|SetOverlayEnabled false))))))
    (:else
      (Variables|OverlayVariables|SetCanActivateOverlay false)
      (Variables|OverlayVariables|SetOverlayEnabled false))))

(event Custom|ChangeLocomotionState_Event
  (params (NewLocomotionState :type E_LocomotionStates%20Enum :default "NewEnumerator0") (PrevLocomotionState :type E_LocomotionStates%20Enum :default "NewEnumerator0"))
  (bind _overlayenabledforlocomotionstate (Variables|Overlay|GetOverlayEnabledForLocomotionState))
  (bind _returnvalue (Utilities|Array|ContainsItem _overlayenabledforlocomotionstate NewLocomotionState))
  (if (Variables|OverlayVariables|GetCanActivateOverlay)
    (if (Math|Boolean|NotEqual(Boolean) (Variables|OverlayVariables|GetOverlayEnabled) _returnvalue)
      (Variables|OverlayVariables|SetOverlayEnabled _returnvalue))))